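; Motion controller component for the VR mod that drives its relative transform from tracked XR hand controller data.
; On BeginPlay it picks the left or right hand from MotionSource.
; Each tick it reads that hand's controller data and, if valid, teleports itself to the aim pose for LeftAim or RightAim sources, otherwise to the grip pose.
; A camera-rotation correction of the location is left disconnected.
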(event `self.ReceiveBeginPlay`
  (bind _motionsource (`self.MotionSource`))
  (if (or (== _motionsource "Left") (== _motionsource "LeftAim"))
    (set `self.ControllerHand` "Left")
    (else
      (set `self.ControllerHand` "Right"))))

(event `self.ReceiveTick`
  (params (DeltaSeconds :type "Float (single-precision)"))
  (bind _motionsource (`self.MotionSource`))
  (bind _motioncontrollerdata (`HeadMountedDisplayFunctionLibrary.GetMotionControllerData` (`self.GetOwner`) (`self.ControllerHand`)))
  (bind ((`bValid` _bvalid) (`GripPosition` _gripposition) (`GripRotation` _griprotation) (`AimPosition` _aimposition) (`AimRotation` _aimrotation)) (break `XRMotionControllerData` _motioncontrollerdata))
  (if _bvalid
    (set `self.Grip Position` _gripposition)
    (set `self.Grip Rotation` _griprotation)
    (set `self.Aim Position` _aimposition)
    (set `self.Aim Rotation` _aimrotation)
    (if (or (== _motionsource "LeftAim") (== "RightAim" _motionsource))
      (set `self.New Location` (`self.Aim Position`))
      (set `self.New Rotation` (`KismetMathLibrary.Quat_Rotator` (`self.Aim Rotation`)))
      (else
        (set `self.New Location` (`self.Grip Position`))
        (set `self.New Rotation` (`KismetMathLibrary.Quat_Rotator` (`self.Grip Rotation`)))))
    (`self.K2_SetRelativeLocationAndRotation` (`self.New Location`) (`self.New Rotation`) false true)))